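; BP_BurningComponent is a damage zone that repeatedly hurts actors inside its Box collision volume.
; Begin overlap adds actors that have a BP_HealthComponent to the ActorToDamage array, and end overlap removes them.
; A looping timer started on BeginPlay applies BaseDamage to every actor in that array on each tick.
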(event OnComponentBeginOverlap(Box)
  (params (OverlappedComponent :type Primitive%20Component%20Object%20Reference) (OtherActor :type Actor%20Object%20Reference) (OtherComp :type Primitive%20Component%20Object%20Reference) (OtherBodyIndex :type Integer) (bFromSweep :type Boolean) (SweepResult :type Hit%20Result%20Structure%20%28by%20ref%29))
  (Utilities|IsValid (Actor|GetComponentbyClass OtherActor "/Game/Extras/BP_HealthComponent.BP_HealthComponent_C")
    (:Is%20Valid
      (Utilities|Array|Add (Variables|Default|GetActorToDamage) OtherActor))))

(event OnComponentEndOverlap(Box)
  (params (OverlappedComponent :type Primitive%20Component%20Object%20Reference) (OtherActor :type Actor%20Object%20Reference) (OtherComp :type Primitive%20Component%20Object%20Reference) (OtherBodyIndex :type Integer))
  (bind _actortodamage (Variables|Default|GetActorToDamage))
  (bind _returnvalue (Utilities|Array|FindItem _actortodamage OtherActor))
  (if (>= _returnvalue 0)
    (Utilities|Array|RemoveIndex (Variables|Default|GetActorToDamage) _returnvalue)))

(event Custom|DamageTick
  (for _array_element (Variables|Default|GetActorToDamage)
    (Game|Damage|ApplyDamage _array_element (Variables|Default|GetBase%20Damage) 0 0)))

(event EventBeginPlay
  (Utilities|Time|SetTimerbyEvent (delegate Custom|DamageTick) 0.0 true))

(fn ConstructionScript)