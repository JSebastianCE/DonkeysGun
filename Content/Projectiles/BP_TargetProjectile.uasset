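; BP_TargetProjectile is a projectile Blueprint that damages whatever actor it hits.
; On BeginPlay it binds DamageEnemy to the OnProjectileImpact dispatcher.
; DamageEnemy sends a TakeDamage interface message to the hit actor with a fixed damage amount and type in an SDamageinfo struct, with no check on what was hit.
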(event Custom|DamageEnemy
  (params (Other%20Actor :type Actor%20Object%20Reference) (Hit :type Hit%20Result%20Structure))
  (Class|BPIDamagable|TakeDamage(Message) Other%20Actor (Utilities|Struct|MakeS_Damageinfo 1e+01 "NewEnumerator1" "NewEnumerator1")))

(event EventBeginPlay
  (|CallParentFunction)
  (EventDispatchers|BindEventtoOnProjectileImpact (delegate Custom|DamageEnemy)))

(event Collision|EventActorBeginOverlap
  (params (OtherActor :type Actor%20Object%20Reference))
  (|CallParentFunction OtherActor) ; This node is disabled and will not be called.\nDrag off pins to build functionality.
)

(event EventTick
  (params (DeltaSeconds :type Float%20%28single-precision%29))
  (|CallParentFunction DeltaSeconds) ; This node is disabled and will not be called.\nDrag off pins to build functionality.
)

(fn ConstructionScript
  (|CallParentFunction))